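; Game mode for a spaceship game that lays out the background and shows the end-game screen.
; On BeginPlay it spawns ten Background_BP tiles, chaining each at the previous tile's AttachPoint via NextSpawnPoint.
; Tick polls Finished and, after a two-second Delay, adds an EndGame_Widget to the viewport, repeating while the flag stays set.
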(event EventBeginPlay
  (for _index (range 0 9)
    (CallFunction|AddBackgroundTile)))

(event EventTick
  (params (DeltaSeconds :type Float%20%28single-precision%29))
  (if (Variables|Default|Getfinished)
    (Utilities|FlowControl|Delay 2.0)
    (bind _returnvalue (UserInterface|CreateWidget "/Game/UI/EndGame_Widget.EndGame_Widget_C"))
    (UserInterface|Viewport|AddtoViewport _returnvalue 0)))

(fn ConstructionScript)

(fn AddBackgroundTile
  (bind _returnvalue (Game|SpawnActorfromClass "/Game/Blueprints/Background_BP.Background_BP_C" (Math|Transform|MakeTransform (Variables|Default|GetNextSpawnPoint)) "Undefined" 0 0))
  (bind _asbackground_bp (Utilities|Casting|CastToBackground_BP _returnvalue))
  (Variables|Default|SetNextSpawnPoint (Transformation|GetWorldLocation (Variables|/Game/Blueprints/Background_BP.Background_BP_C|GetAttachPoint _asbackground_bp))))